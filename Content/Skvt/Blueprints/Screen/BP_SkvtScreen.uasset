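; Screen actor that displays a WBP_SkvtWeb web page through its Webpage widget component.
; On BeginPlay, Initialize casts the component's widget to WBP_SkvtWeb and caches it in WebpageRef.
; ToggleOn shows or hides the Webpage component without affecting its children, and the TurnOff event calls it to hide the page.
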(event EventBeginPlay
  (CallFunction|Initialize))

(event Collision|EventActorBeginOverlap
  (params (OtherActor :type Actor%20Object%20Reference)))

(event EventTick
  (params (DeltaSeconds :type Float%20%28single-precision%29)))

(event EventTurnOff
  (CallFunction|Toggleon false))

(fn ConstructionScript)

(fn Initialize
  (bind _aswbp_skvt_web (Utilities|Casting|CastToWBP_SkvtWeb (UserInterface|GetWidget (Variables|Default|GetWebpage))))
  (Variables|Default|SetWebpageRef _aswbp_skvt_web))

(fn Toggleon
  (params (TurnOn :type Boolean))
  (Rendering|SetVisibility (Variables|Default|GetWebpage) TurnOn false))