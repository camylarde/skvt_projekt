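; Player controller that lets the player cycle possession between BP_SkvtBaseChar characters in the level.
; BeginPlay adds the default, pawn-swap and camera Enhanced Input mapping contexts.
; IA_Swap gathers all such characters and possesses the one after the current pawn, wrapping to the first via GetCharacterToPossess.
; Disconnected leftovers hold an older inline swap and a deprecated player-mappable config setup.
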(event Input|EnhancedActionEvents|EnhancedInputActionIA_Swap
  (params (ActionValue :type Boolean) (ElapsedSeconds :type Float%20%28double-precision%29) (TriggeredSeconds :type Float%20%28double-precision%29) (InputAction :type Input%20Action%20Object%20Reference :default "/Game/Skvt/Characters/Input/Actions/IA_Swap.IA_Swap"))
  (:Triggered
    (bind _outactors (Actor|GetAllActorsOfClass "/Game/Skvt/Characters/BP_SkvtBaseChar.BP_SkvtBaseChar_C"))
    (Pawn|Possess (CallFunction|GetCharactertoPossess _outactors))))

(event EventBeginPlay
  (bind _self self)
  (bind _returnvalue (PlayerController|LocalPlayerSubsystems|GetEnhancedInputLocalPlayerSubsystem _self))
  (Utilities|IsValid _returnvalue
    (:Is%20Valid
      (Input|AddMappingContext _returnvalue "/Game/ThirdPerson/Input/IMC_Default.IMC_Default" 0 "(bIgnoreAllPressedKeysUntilRelease=True,bForceImmediately=False)")
      (Input|AddMappingContext _returnvalue "/Game/Skvt/Characters/Input/IMC_SwapPawn.IMC_SwapPawn" 0 "(bIgnoreAllPressedKeysUntilRelease=True,bForceImmediately=False)")
      (Input|AddMappingContext _returnvalue "/Game/Skvt/Characters/Input/IMC_Camera.IMC_Camera" 0 "(bIgnoreAllPressedKeysUntilRelease=True,bForceImmediately=False)"))))

(fn ConstructionScript)

(fn GetCharactertoPossess
  (params (Pawn%20array :type Array%20of%20BP%20Skvt%20Base%20Char%20Object%20References))
  (bind _asbp_skvt_base_char (Utilities|Casting|CastToBP_SkvtBaseChar (Pawn|GetControlledPawn)))
  (if (Utilities|Array|IsValidIndex Pawn%20array (+ (Utilities|Array|FindItem Pawn%20array _asbp_skvt_base_char) 1))
    (return (Utilities|Array|Get(acopy) Pawn%20array (+ (Utilities|Array|FindItem Pawn%20array _asbp_skvt_base_char) 1)))
    (else
      (return (Utilities|Array|Get(acopy) Pawn%20array)))))